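; Game mode that tracks progression through a list of missions and their tasks.
; Each Tick refreshes the current mission and task from saved indices, though the refresh is guarded by a 0 > Missions length check.
; Ordered missions advance task by task, completing after the last.
; Unordered missions scan all tasks with a breakable loop before being marked complete and advancing the mission index.
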(event Custom|UpdateCurrentMission
  (bind _currentmissionindex (Variables|Default|GetcurrentMissionIndex))
  (bind _missions (Variables|Default|Getmissions))
  (bind _output (Utilities|Array|Get(acopy) _missions _currentmissionindex))
  (if (> 0 (Utilities|Array|Length (Variables|Default|Getmissions)))
    (bind _output_get (Variables|Default|SetcurrentMissions _output))
    (Variables|/Game/Blueprints/ProgressionSystem/Mission.Mission_C|SetcurrentTask _output_get (Utilities|Array|Get(acopy) (Variables|/Game/Blueprints/ProgressionSystem/Mission.Mission_C|Gettasks _output_get) (Variables|/Game/Blueprints/ProgressionSystem/Mission.Mission_C|GetcurrentTaskIndex _output)))))

(event Custom|Break%20Task%20Loop
  (bind _currentmissions (Variables|Default|GetcurrentMissions))
  (Utilities|Array|ForEachLoopwithBreak (Variables|/Game/Blueprints/ProgressionSystem/Mission.Mission_C|Gettasks _currentmissions)) ; enters at Break
)

(event EventTick
  (params (DeltaSeconds :type Float%20%28single-precision%29))
  (bind _currentmissions (Variables|Default|GetcurrentMissions))
  (bind _currentmissions_2 (Variables|Default|GetcurrentMissions))
  (bind _currentmissions_3 (Variables|Default|GetcurrentMissions))
  (bind _currentmissions_4 (Variables|Default|GetcurrentMissions))
  (CallFunction|UpdateCurrentMission)
  (if (!= 0 _currentmissions)
    (if (Variables|/Game/Blueprints/ProgressionSystem/Mission.Mission_C|GettaskCompletionInOrder _currentmissions)
      (if (.completed (Utilities|Struct|BreakMissionTask (Variables|/Game/Blueprints/ProgressionSystem/Mission.Mission_C|GetcurrentTask (Variables|Default|GetcurrentMissions))))
        (if (< (Variables|/Game/Blueprints/ProgressionSystem/Mission.Mission_C|GetcurrentTaskIndex _currentmissions_2) (- (Utilities|Array|Length (Variables|/Game/Blueprints/ProgressionSystem/Mission.Mission_C|Gettasks _currentmissions_2)) 1))
          (Math|Integer|IncrementInt (Variables|/Game/Blueprints/ProgressionSystem/Mission.Mission_C|GetcurrentTaskIndex _currentmissions_3))
          (else
            (Default|SetCompleted _currentmissions_3 true)
            (Math|Integer|IncrementInt (Variables|Default|GetcurrentMissionIndex)))))
      (else
        (bind _array_element (Utilities|Array|ForEachLoopwithBreak (Variables|/Game/Blueprints/ProgressionSystem/Mission.Mission_C|Gettasks _currentmissions_4))
          (:LoopBody
            (if (not (.completed (Utilities|Struct|BreakMissionTask _array_element)))
              (CallFunction|BreakTaskLoop)))
          (:Completed
            (Default|SetCompleted _currentmissions_4 true)
            (Math|Integer|IncrementInt (Variables|Default|GetcurrentMissionIndex))))))))

(fn ConstructionScript)