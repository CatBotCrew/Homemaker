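; Mission handler that steps through an array of missions and their tasks, tracking progression by index.
; Every Tick it refreshes the current mission and task from those indices.
; Ordered missions advance task by task as each completes, then complete and move to the next mission.
; Unordered missions scan tasks, breaking at the first unfinished one, though completion and advance follow the loop even after a break.
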(event Custom|Update%20Current%20Mission
  (bind _currentmissionindex (Variables|Default|GetcurrentMissionIndex))
  (bind _missions (Variables|Default|Getmissions))
  (bind _output (Utilities|Array|Get(acopy) _missions _currentmissionindex))
  (bind _output_get (Variables|Default|SetcurrentMission _output))
  (Variables|/Game/Blueprints/ProgressionSystem/Mission.Mission_C|SetcurrentTask _output_get (Utilities|Array|Get(acopy) (Variables|/Game/Blueprints/ProgressionSystem/Mission.Mission_C|Gettasks _output_get) (Variables|/Game/Blueprints/ProgressionSystem/Mission.Mission_C|GetcurrentTaskIndex _output))))

(event Custom|Break%20Task%20Loop
  (bind _currentmission (Variables|Default|GetcurrentMission))
  (Utilities|Array|ForEachLoopwithBreak (Variables|/Game/Blueprints/ProgressionSystem/Mission.Mission_C|Gettasks _currentmission)) ; enters at Break
)

(event EventTick
  (params (DeltaSeconds :type Float%20%28single-precision%29))
  (bind _currentmission (Variables|Default|GetcurrentMission))
  (bind _currentmission_2 (Variables|Default|GetcurrentMission))
  (bind _currentmission_3 (Variables|Default|GetcurrentMission))
  (bind _currentmission_4 (Variables|Default|GetcurrentMission))
  (CallFunction|UpdateCurrentMission)
  (if (!= 0 _currentmission)
    (if (Variables|/Game/Blueprints/ProgressionSystem/Mission.Mission_C|GettaskCompletionInOrder _currentmission)
      (if (.completed (Utilities|Struct|BreakMissionTask (Variables|/Game/Blueprints/ProgressionSystem/Mission.Mission_C|GetcurrentTask (Variables|Default|GetcurrentMission))))
        (if (< (Variables|/Game/Blueprints/ProgressionSystem/Mission.Mission_C|GetcurrentTaskIndex _currentmission_2) (- (Utilities|Array|Length (Variables|/Game/Blueprints/ProgressionSystem/Mission.Mission_C|Gettasks _currentmission_2)) 1))
          (Math|Integer|IncrementInt (Variables|/Game/Blueprints/ProgressionSystem/Mission.Mission_C|GetcurrentTaskIndex _currentmission_3))
          (else
            (Default|SetCompleted _currentmission_3 true)
            (Math|Integer|IncrementInt (Variables|Default|GetcurrentMissionIndex)))))
      (else
        (bind _array_element (Utilities|Array|ForEachLoopwithBreak (Variables|/Game/Blueprints/ProgressionSystem/Mission.Mission_C|Gettasks _currentmission_4))
          (:LoopBody
            (if (not (.completed (Utilities|Struct|BreakMissionTask _array_element)))
              (CallFunction|BreakTaskLoop)))
          (:Completed
            (Default|SetCompleted _currentmission_4 true)
            (Math|Integer|IncrementInt (Variables|Default|GetcurrentMissionIndex))))))))

(fn ConstructionScript)