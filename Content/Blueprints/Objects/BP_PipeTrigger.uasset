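; BP_PipeTrigger is an interactable valve that, while water is running, plays a one-time scripted pipe cinematic and then locks.
; Activation stops the Tap's tick, disables input and blends the view to itself, then sequences water, steam, sounds and radio voice lines with delays.
; Tick, enabled mid-sequence, sinks the DishTower and raises the WaterPuddle toward construction-script heights.
; Glow events toggle the valve's custom-depth highlight.
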(event EventActivateGlow
  (if (and (Components|Activation|IsActive (Variables|/Script/Engine.Emitter|GetParticleSystemComponent (Variables|Default|Getwater))) (not (Variables|Default|Getlocked)))
    (Rendering|SetRenderCustomDepth (Variables|/Script/Engine.StaticMeshActor|GetStaticMeshComponent (Variables|Default|Getvalve)) true)))

(event EventTick
  (params (DeltaSeconds :type Float%20%28single-precision%29))
  (bind _dishtower (Variables|Default|GetdishTower))
  (bind _waterpuddle (Variables|Default|GetwaterPuddle))
  (bind _returnvalue (Transformation|GetActorLocation _waterpuddle))
  (bind _returnvalue_2 (Transformation|GetActorLocation _dishtower))
  (Transformation|SetActorLocation (Variables|Default|GetdishTower) (Math|Interpolation|VInterptoConstant (Transformation|GetActorLocation (Variables|Default|GetdishTower)) (Math|Vector|MakeVector (.x _returnvalue_2) (.y _returnvalue_2) (Variables|Default|GetnewDishZ)) (Utilities|Time|GetWorldDeltaSeconds) 2e+01) false false)
  (Transformation|SetActorLocation (Variables|Default|GetwaterPuddle) (Math|Interpolation|VInterptoConstant (Transformation|GetActorLocation (Variables|Default|GetwaterPuddle)) (Math|Vector|MakeVector (.x _returnvalue) (.y _returnvalue) (Variables|Default|GetnewPuddleZ)) (Utilities|Time|GetWorldDeltaSeconds) 2e+01) false false))

(event EventOnActivation
  (if (and (Components|Activation|IsActive (Variables|/Script/Engine.Emitter|GetParticleSystemComponent (Variables|Default|Getwater))) (not (Variables|Default|Getlocked)))
    (Actor|Tick|SetActorTickEnabled (Variables|Default|Gettap))
    (bind _asbp_player_character (Utilities|Casting|CastToBP_PlayerCharacter (Game|Player|GetPlayerPawn 0)))
    (Variables|/Game/Blueprints/Player/BP_PlayerCharacter.BP_PlayerCharacter_C|SetactiveInteractableObject _asbp_player_character 0)
    (Variables|/Game/Blueprints/Player/BP_PlayerCharacter.BP_PlayerCharacter_C|SetCurrentInteractableObject _asbp_player_character 0)
    (Input|DisableInput (Game|GetPlayerCharacter 0) (Game|GetPlayerController 0))
    (Game|Player|SetViewTargetwithBlend (Game|GetPlayerController 0) self 2.0 "VTBlend_EaseInOut" 3.0 false)
    (Utilities|FlowControl|Delay 3.0)
    (Effects|Components|ParticleSystem|SetTemplate (Variables|/Script/Engine.Emitter|GetParticleSystemComponent (Variables|Default|Getwater)) "/Game/StarterContent/Particles/P_WaterBig.P_WaterBig")
    (Audio|PlaySound2D "/Game/Audio/SoundEffects/Chapter_One/WaterDripping_Cue.WaterDripping_Cue" 1.0 1.0 0.0 0 0)
    (Utilities|FlowControl|Delay 1.0)
    (Components|Activation|Activate (Variables|/Script/Engine.Emitter|GetParticleSystemComponent (Variables|Default|Getsteam)) true)
    (Audio|PlaySound2D "/Game/Audio/SoundEffects/Chapter_One/WaterWashingDishesFlushing_Cue.WaterWashingDishesFlushing_Cue" 1.0 1.0 0.0 0 0)
    (Utilities|FlowControl|Delay 2.0)
    (Actor|Tick|SetActorTickEnabled true)
    (Default|PlaySound (Variables|Default|Getradio) "/Game/Audio/Radio/VoiceLines/VoiceLine_OhMyStars_Cue.VoiceLine_OhMyStars_Cue")
    (Utilities|FlowControl|Delay 4.0)
    (Game|Player|SetViewTargetwithBlend (Game|GetPlayerController 0) (Game|GetPlayerCharacter 0) 2.0 "VTBlend_EaseInOut" 3.0 false)
    (Utilities|FlowControl|Delay 2.0)
    (Input|EnableInput (Game|GetPlayerCharacter 0) (Game|GetPlayerController 0))
    (Actor|Tick|SetActorTickEnabled false)
    (Variables|Default|Setlocked true)
    (Utilities|FlowControl|Delay 1e+01)
    (Default|PlaySound (Variables|Default|Getradio) "/Game/Audio/Radio/VoiceLines/VoiceLine_Pixiemop_Cue.VoiceLine_Pixiemop_Cue")))

(event EventDeactivateGlow
  (Rendering|SetRenderCustomDepth (Variables|/Script/Engine.StaticMeshActor|GetStaticMeshComponent (Variables|Default|Getvalve)) false))

(fn ConstructionScript
  (|CallParentFunction)
  (Variables|Default|SetnewDishZ (- (.z (Transformation|GetActorLocation (Variables|Default|GetdishTower))) 2e+02))
  (Variables|Default|SetnewPuddleZ (+ (.z (Transformation|GetActorLocation (Variables|Default|GetwaterPuddle))) 1e+01)))