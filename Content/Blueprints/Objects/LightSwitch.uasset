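; Light switch actor that toggles its assigned point and spot lights when the player activates it.
; OnActivation draws a debug "Switched" label at the switch, then flips root component visibility on both light arrays, propagating to children.
; BeginPlay reuses that toggle when OffByDefault is set, so it only turns off lights that start visible.
; Glow events switch custom depth rendering on the switch component on and off for highlighting.
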(event EventOnActivation
  ;[1 1 1] Call On Activation Function From Player
  (Rendering|Debug|DrawDebugString (Transformation|GetWorldLocation (Variables|Default|GetSwitch)) "Switched" 0 "(R=0.021456,G=1.000000,B=0.000000,A=1.000000)" 5.0)
  (for _array_element (Variables|LightSettings|GetPointLights)
    (Rendering|ToggleVisibility (Variables|/Script/Engine.Actor|GetRootComponent _array_element) true))
  (for _array_element_2 (Variables|LightSettings|GetSpotLights)
    (Rendering|ToggleVisibility (Variables|/Script/Engine.Actor|GetRootComponent _array_element_2) true)))

(event EventBeginPlay
  (if (Variables|LightSettings|GetOffByDefault)
    (for _array_element (Variables|LightSettings|GetPointLights)
      (Rendering|ToggleVisibility (Variables|/Script/Engine.Actor|GetRootComponent _array_element) true))
    (for _array_element_2 (Variables|LightSettings|GetSpotLights)
      (Rendering|ToggleVisibility (Variables|/Script/Engine.Actor|GetRootComponent _array_element_2) true))))

(event EventActivateGlow
  (Rendering|SetRenderCustomDepth (Variables|Default|GetSwitch) true))

(event EventDeactivateGlow
  (Rendering|SetRenderCustomDepth (Variables|Default|GetSwitch) false))

(fn ConstructionScript
  (|CallParentFunction))