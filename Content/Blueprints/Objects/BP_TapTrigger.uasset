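; BP_TapTrigger is an interactable tap that, once the player holds the emptied sandwich plate, plays a dish-tower and water cutscene.
; Tick checks the player's attached actors for that plate, and custom depth highlights the tap when usable.
; Activation hides the plate, disables input and blends the view to itself.
; Timed delays start the tower's interpolated rise and the water particles, then restore view and control.
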(event EventTick
  (params (DeltaSeconds :type Float%20%28single-precision%29))
  (bind _sandwhich (Variables|Default|Getsandwhich))
  (bind _dishtower (Variables|Default|GetdishTower))
  (bind _returnvalue (Transformation|GetActorLocation _dishtower))
  (for _array_element (Actor|GetAttachedActors (Game|GetPlayerCharacter 0))
    (if (and (== _array_element _sandwhich) (not (Rendering|IsVisible (Variables|/Game/Blueprints/Objects/BP_MovableSandwhich.BP_MovableSandwhich_C|GetSandwhich _sandwhich))))
      (Variables|Default|SetholdingPlate true)))
  (if (Variables|Default|GetraiseDishes)
    (Transformation|SetActorLocation (Variables|Default|GetdishTower) (Math|Interpolation|VInterptoConstant (Transformation|GetActorLocation (Variables|Default|GetdishTower)) (Math|Vector|MakeVector (.x _returnvalue) (.y _returnvalue) (Variables|Default|GetnewDishZ)) (Utilities|Time|GetWorldDeltaSeconds) 2e+01) false false)))

(event EventOnActivation
  (if (and (not (Components|Activation|IsActive (Variables|/Script/Engine.Emitter|GetParticleSystemComponent (Variables|Default|Getwater)))) (Variables|Default|GetholdingPlate))
    (Rendering|SetActorHiddenInGame (Variables|Default|Getsandwhich) true)
    (bind _asbp_player_character (Utilities|Casting|CastToBP_PlayerCharacter (Game|Player|GetPlayerPawn 0)))
    (Variables|/Game/Blueprints/Player/BP_PlayerCharacter.BP_PlayerCharacter_C|SetactiveInteractableObject _asbp_player_character 0)
    (Variables|/Game/Blueprints/Player/BP_PlayerCharacter.BP_PlayerCharacter_C|SetCurrentInteractableObject _asbp_player_character 0)
    (CallFunction|Deactivate)
    (Input|DisableInput (Game|GetPlayerCharacter 0) (Game|GetPlayerController 0))
    (Game|Player|SetViewTargetwithBlend (Game|GetPlayerController 0) self 2.0 "VTBlend_EaseInOut" 3.0 false)
    (Utilities|FlowControl|Delay 3.0)
    (Variables|Default|SetraiseDishes true)
    (Utilities|FlowControl|Delay 3.0)
    (Components|Activation|Activate (Variables|/Script/Engine.Emitter|GetParticleSystemComponent (Variables|Default|Getwater)) true)
    (Utilities|FlowControl|Delay 2.0)
    (Game|Player|SetViewTargetwithBlend (Game|GetPlayerController 0) (Game|GetPlayerCharacter 0) 2.0 "VTBlend_EaseInOut" 3.0 false)
    (Utilities|FlowControl|Delay 2.0)
    (Input|EnableInput (Game|GetPlayerCharacter 0) (Game|GetPlayerController 0))))

(event EventActivateGlow
  (if (and (not (Components|Activation|IsActive (Variables|/Script/Engine.Emitter|GetParticleSystemComponent (Variables|Default|Getwater)))) (Variables|Default|GetholdingPlate))
    (Rendering|SetRenderCustomDepth (Variables|/Script/Engine.StaticMeshActor|GetStaticMeshComponent (Variables|Default|Gettap)) true)))

(event EventDeactivateGlow
  (Rendering|SetRenderCustomDepth (Variables|/Script/Engine.StaticMeshActor|GetStaticMeshComponent (Variables|Default|Gettap)) false))

(fn ConstructionScript
  (|CallParentFunction)
  (Variables|Default|SetnewDIshZ (+ (.z (Transformation|GetActorLocation (Variables|Default|GetdishTower))) 8e+01)))