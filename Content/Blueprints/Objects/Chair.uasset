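; Interactable chair object that can be activated and highlighted in the game.
; Activation plays a non-looping animation on the first skeletal mesh component of player 0's pawn, with no animation asset shown.
; Glow events toggle custom depth rendering on the Chair component to switch the highlight on and off.
; The construction script only calls its parent's version.
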(event EventActivateGlow
  (Rendering|SetRenderCustomDepth (Variables|Default|GetChair) true))

(event EventDeactivateGlow
  (Rendering|SetRenderCustomDepth (Variables|Default|GetChair) false))

(event EventOnActivation
  (Components|Animation|PlayAnimation (Actor|GetComponentbyClass (Game|Player|GetPlayerPawn 0) "/Script/Engine.SkeletalMeshComponent") 0 false))

(fn ConstructionScript
  (|CallParentFunction))