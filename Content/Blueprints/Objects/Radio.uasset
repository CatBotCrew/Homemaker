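; Interactive radio that plays a sound at its mesh's location and pulses in scale with the audio.
; Player activation toggles pause, starting from PlayOnStart.
; Tick averages seven frequency band magnitudes from output analysis, which is not tied to its own sound, and interpolates mesh scale only above Threshold.
; Glow events toggle custom depth rendering for highlighting.
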(event EventTick
  (params (DeltaSeconds :type Float%20%28single-precision%29))
  (bind _staticmesh (Variables|Default|GetStaticMesh))
  (Variables|Default|SetsizeModifier 0.0)
  (bind _magnitudes (Class|AudioMixerBlueprintLibrary|GetMagnitudeforFrequencies (Utilities|Array|MakeArray 6e+01 2.5e+02 5e+02 2e+03 4e+03 6e+03 2e+04) 0))
  (bind _output_get (Variables|RadioSettings|Setmagnitudes _magnitudes))
  (for _array_element _output_get
    (Variables|Default|SetsizeModifier (+ _array_element (Variables|Default|GetsizeModifier))))
  (bind _output_get_2 (Variables|Default|SetsizeModifier (/ (Variables|Default|GetsizeModifier) (Math|Conversions|ToFloat(Integer) (Utilities|Array|Length _magnitudes)))))
  (if (> (Math|Float|NormalizetoRange _output_get_2 0.0 1.0) (Variables|RadioSettings|Getthreshold))
    (Transformation|SetRelativeScale3D _staticmesh (Math|Interpolation|VInterpTo (Variables|/Script/Engine.SceneComponent|GetRelativeScale3D _staticmesh) (Math|Vector|MakeVector (+ (* (Math|Float|NormalizetoRange _output_get_2 0.0 1.0) (Variables|RadioSettings|GetscalingStrenght)) 1.0) (+ (* (Math|Float|NormalizetoRange _output_get_2 0.0 1.0) (Variables|RadioSettings|GetscalingStrenght)) 1.0) (+ (* (Math|Float|NormalizetoRange _output_get_2 0.0 1.0) (Variables|RadioSettings|GetscalingStrenght)) 1.0)) DeltaSeconds (Variables|RadioSettings|GetscalingSpeed)))))

(event EventOnActivation
  ;[1 1 1] Call On Activation Function From Player
  (Rendering|Debug|DrawDebugString (Transformation|GetWorldLocation (Variables|Default|GetStaticMesh)) "Play" 0 "(R=0.021456,G=1.000000,B=0.000000,A=1.000000)" 5.0)
  (if (Variables|Default|Getplaying)
    (Class|AudioComponent|SetPaused (stale EventBeginPlay _returnvalue) true)
    (Variables|Default|Setplaying false)
    (else
      (Class|AudioComponent|SetPaused (stale EventBeginPlay _returnvalue) false)
      (Variables|Default|Setplaying true))))

(event EventBeginPlay
  (bind _playonstart (Variables|RadioSettings|GetplayOnStart))
  (Class|AudioMixerBlueprintLibrary|StartAnalyzingOutput 0)
  (Input|EnableInput (Game|GetPlayerController 0))
  (bind _returnvalue (Audio|SpawnSoundatLocation (Variables|Default|Getsound) (Transformation|GetWorldLocation (Variables|Default|GetStaticMesh)) "0, 0, 0" 1.0 1.0 0.0 0 0))
  (Class|AudioComponent|SetPaused _returnvalue (not _playonstart))
  (Variables|Default|Setplaying _playonstart))

(event EventActivateGlow
  (Rendering|SetRenderCustomDepth (Variables|Default|GetStaticMesh) true))

(event EventDeactivateGlow
  (Rendering|SetRenderCustomDepth (Variables|Default|GetStaticMesh) false))

(fn ConstructionScript
  (|CallParentFunction))