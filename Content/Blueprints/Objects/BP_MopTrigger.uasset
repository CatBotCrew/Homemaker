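; BP_MopTrigger is an interactable that plays a scripted breakdown sequence and then returns to the main menu, available only while PipeTrigger is locked.
; Activation blends the view to itself and bursts three water effects in timed succession with pipe-breaking sounds.
; The view then blends to the Radio, which stops amid electrical effects and a break sound before MainMenu loads.
; Glow events toggle custom depth for highlighting, enabling it under the same lock condition.
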(event EventOnActivation
  (if (Variables|/Game/Blueprints/Objects/BP_PipeTrigger.BP_PipeTrigger_C|Getlocked (Variables|Default|GetpipeTrigger))
    (Audio|PlaySound2D "/Game/Audio/SoundEffects/Chapter_One/PipePressureBuildBreak_Cue.PipePressureBuildBreak_Cue" 1.0 1.0 0.0 0 0)
    (Game|Player|SetViewTargetwithBlend (Game|GetPlayerController 0) self 1.0 "VTBlend_EaseInOut" 2.0 false)
    (Utilities|FlowControl|Delay 1.0)
    (Components|Activation|Activate (Variables|Default|GetWater_1) false)
    (Audio|PlaySound2D "/Game/Audio/SoundEffects/Chapter_One/WAV/PipeBreaking_0.PipeBreaking_0" 1.0 1.0 0.0 0 0)
    (Utilities|FlowControl|Delay 1.0)
    (Components|Activation|Activate (Variables|Default|GetWater_2) false)
    (Audio|PlaySound2D "/Game/Audio/SoundEffects/Chapter_One/WAV/PipeBreaking_1.PipeBreaking_1" 1.0 1.0 0.0 0 0)
    (Utilities|FlowControl|Delay 1.0)
    (Components|Activation|Activate (Variables|Default|GetWater_3) false)
    (Audio|PlaySound2D "/Game/Audio/SoundEffects/Chapter_One/WAV/PipeBreaking_2.PipeBreaking_2" 1.0 1.0 0.0 0 0)
    (Utilities|FlowControl|Delay 1.0)
    (Game|Player|SetViewTargetwithBlend (Game|GetPlayerController 0) (Variables|Default|Getradio) 1.0 "VTBlend_EaseInOut" 2.0 false)
    (Utilities|FlowControl|Delay 1.0)
    (Default|Stop (Variables|Default|Getradio))
    (Components|Activation|Activate (Variables|Default|GetElectricity) false)
    (Audio|PlaySound2D "/Game/Audio/SoundEffects/Chapter_One/RadioBreak_Cue.RadioBreak_Cue" 1.0 1.0 0.0 0 0)
    (Utilities|FlowControl|Delay 6.0)
    (Game|OpenLevel(byName) "MainMenu")))

(event EventActivateGlow
  (if (Variables|/Game/Blueprints/Objects/BP_PipeTrigger.BP_PipeTrigger_C|Getlocked (Variables|Default|GetpipeTrigger))
    (Rendering|SetRenderCustomDepth (Variables|Default|GetStaticMesh) true)))

(event EventDeactivateGlow
  (Rendering|SetRenderCustomDepth (Variables|Default|GetStaticMesh) false))

(fn ConstructionScript
  (|CallParentFunction))