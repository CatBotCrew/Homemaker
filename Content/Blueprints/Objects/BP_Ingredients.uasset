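; BP_Ingredients is an interactable that tracks the five sandwich ingredients and plays the sandwich-making sequence once all are collected.
; Tick reveals meshes matching the game instance's ZuccedInItems, then sets Completed and stops ticking at five items.
; Completed enables custom-depth glow and activation until Locked.
; Activation blends the camera here, plays audio, reveals the sandwich after a delay, returns the view, locks, and triggers a Radio voice line.
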(event EventTick
  (params (DeltaSeconds :type Float%20%28single-precision%29))
  (bind _ashomemaker__gi (Utilities|Casting|CastToHomemaker-GI (Game|GetGameInstance)))
  (for _array_element (Variables|/Game/Blueprints/Homemaker-GI.Homemaker-GI_C|GetzuccedInItems _ashomemaker__gi)
    (switch name _array_element
      (:Lettuce
        (Rendering|SetVisibility (Variables|Default|GetLettuce) true false))
      (:Ham
        (Rendering|SetVisibility (Variables|Default|GetHam) true false))
      (:Cheese
        (Rendering|SetVisibility (Variables|Default|GetCheese) true false))
      (:Tomato
        (Rendering|SetVisibility (Variables|Default|GetTomato) true false))
      (:Mayo
        (Rendering|SetVisibility (Variables|Default|GetMayo) true false))))
  (if (== (Utilities|Array|Length (Variables|/Game/Blueprints/Homemaker-GI.Homemaker-GI_C|GetzuccedInItems _ashomemaker__gi)) 5)
    (Variables|Default|Setcompleted true)
    (Actor|Tick|SetActorTickEnabled false)))

(event EventActivateGlow
  (if (and (Variables|Default|Getcompleted) (not (Variables|Default|Getlocked)))
    (for _array_element (Actor|GetComponentsByClass "/Script/Engine.StaticMeshComponent")
      (Rendering|SetRenderCustomDepth _array_element true))))

(event EventDeactivateGlow
  (for _array_element (Actor|GetComponentsByClass "/Script/Engine.StaticMeshComponent")
    (Rendering|SetRenderCustomDepth _array_element false)))

(event EventOnActivation
  (if (and (Variables|Default|Getcompleted) (not (Variables|Default|Getlocked)))
    (Game|Player|SetViewTargetwithBlend (Game|GetPlayerController 0) self 1.0 "VTBlend_EaseInOut" 2.0 false)
    (Audio|PlaySound2D "/Game/Audio/SoundEffects/Chapter_One/MakingSandwich_Cue.MakingSandwich_Cue" 1.0 1.0 0.0 0 0)
    (Utilities|FlowControl|Delay 5.5)
    (Rendering|SetVisibility (Variables|/Game/Blueprints/Objects/BP_MovableSandwhich.BP_MovableSandwhich_C|GetSandwhich (Variables|Default|Getsandwhich)) true false)
    (Utilities|FlowControl|Delay 1.0)
    (Game|Player|SetViewTargetwithBlend (Game|GetPlayerController 0) (Game|GetPlayerCharacter 0) 1.0 "VTBlend_EaseInOut" 2.0 false)
    (Variables|Default|Setlocked true)
    (Default|PlaySound (Variables|Default|Getradio) "/Game/Audio/Radio/VoiceLines/VoiceLine_3_Cue.VoiceLine_3_Cue")))

(fn ConstructionScript)