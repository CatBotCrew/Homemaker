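; Interactable sandwich-on-a-plate object that the player can pick up and carry.
; Glow events toggle custom depth on the plate and sandwich for highlighting.
; Activation snaps the actor to the player's ItemHolder, attaches it to the player character and clears the player's active and current interactable references.
; Highlighting and pickup require the sandwich to be visible or FinishedEating to be true.
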(event EventOnActivation
  (if (or (Rendering|IsVisible (Variables|Default|GetSandwhich)) (Variables|Default|GetfinishedEating))
    (bind _asbp_player_character (Utilities|Casting|CastToBP_PlayerCharacter (Game|GetPlayerCharacter 0)))
    (Transformation|SetActorLocation (Transformation|GetWorldLocation (Variables|/Game/Blueprints/Player/BP_PlayerCharacter.BP_PlayerCharacter_C|GetItemHolder _asbp_player_character)) false false)
    (Transformation|AttachActorToActor (Game|GetPlayerCharacter 0) "None" "KeepWorld" "KeepWorld" "KeepWorld" true)
    (bind _asbp_player_character_2 (Utilities|Casting|CastToBP_PlayerCharacter (Game|GetPlayerCharacter 0)))
    (Variables|/Game/Blueprints/Player/BP_PlayerCharacter.BP_PlayerCharacter_C|SetactiveInteractableObject _asbp_player_character_2 0)
    (Variables|/Game/Blueprints/Player/BP_PlayerCharacter.BP_PlayerCharacter_C|SetCurrentInteractableObject _asbp_player_character_2 0)))

(event EventActivateGlow
  (if (or (Rendering|IsVisible (Variables|Default|GetSandwhich)) (Variables|Default|GetfinishedEating))
    (Rendering|SetRenderCustomDepth (Variables|Default|GetPlate) true)))

(event EventDeactivateGlow
  (Rendering|SetRenderCustomDepth (Variables|Default|GetPlate) false))

(fn ConstructionScript
  (|CallParentFunction))