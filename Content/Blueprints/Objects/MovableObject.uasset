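; MovableObject is an interactable physics object that the player can grab and push or pull, and that falls when it loses ground.
; Activation events toggle grabbed state, physics and collision, and while grabbed, Tick applies force from the player's velocity.
; A downward trace finding no nearby ground latches a falling state, which releases the grab, lowers damping and clears constraints every tick.
; Glow events toggle custom depth rendering on the mesh.
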(event Custom|HandleFalling
  (bind _collisionbox (Variables|Default|GetCollisionBox))
  ;[1 1 1] Falling
  (Variables|Default|SetisGrabbed false)
  (Physics|SetSimulatePhysics _collisionbox true)
  (Collision|SetCollisionEnabled _collisionbox "QueryAndPhysics")
  (Variables|Default|SetoriginalLinearDamp (Class|PrimitiveComponent|GetLinearDamping _collisionbox))
  (Variables|Default|SetoriginalAngDamp (Class|PrimitiveComponent|GetAngularDamping _collisionbox))
  (Class|PrimitiveComponent|SetAngularDamping _collisionbox 0.0)
  (Class|PrimitiveComponent|SetLinearDamping _collisionbox 0.01)
  (Class|PrimitiveComponent|SetConstraintMode _collisionbox "None"))

(event EventActivateGlow
  (Rendering|SetRenderCustomDepth (Variables|Default|GetStaticMesh) true))

(event EventTick
  (params (DeltaSeconds :type Float%20%28single-precision%29))
  (bind _staticmesh (Variables|Default|GetStaticMesh))
  (bind _returnvalue (Transformation|GetWorldLocation _staticmesh))
  ;[1 1 1] Tick
  (if (Variables|Default|GetisFalling)
    (CallFunction|HandleFalling)
    (elif (Variables|Default|GetisGrabbed)
      (Physics|AddForce (Variables|Default|GetCollisionBox) (* (Transformation|GetVelocity (Game|GetPlayerCharacter 0)) 5.5) "None" true)
      (bind _outhit (Collision|LineTraceByChannel _returnvalue (+ _returnvalue (* (Math|Vector|GetUpVector _staticmesh) -1e+03)) "TraceTypeQuery1" false 0 "ForOneFrame"))
      (if (.bblockinghit _outhit)
        (if (> (.distance _outhit) 1e+02)
          (Variables|Default|SetisFalling true :!label _label))
        (else
          (goto _label))))))

(event EventOnActivation
  (bind _collisionbox (Variables|Default|GetCollisionBox))
  ;[1 1 1] Activation / Deactivation
  (Variables|Default|SetisGrabbed true)
  (Physics|SetSimulatePhysics _collisionbox true)
  (Collision|SetCollisionEnabled _collisionbox "QueryAndPhysics"))

(event EventAfterActivation
  (bind _collisionbox (Variables|Default|GetCollisionBox))
  ;[1 1 1] Activation / Deactivation
  (Variables|Default|SetisGrabbed false)
  (Physics|SetSimulatePhysics _collisionbox false)
  (Collision|SetCollisionEnabled _collisionbox "QueryOnly"))

(event EventDeactivateGlow
  (Rendering|SetRenderCustomDepth (Variables|Default|GetStaticMesh) false))

(fn ConstructionScript
  (|CallParentFunction))