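; Player character Blueprint that handles interaction with nearby objects and shows health through a screen damage post-process effect.
; Overlapped interactables join an array; each tick the one within angle and distance limits with the smallest angle glows.
; The Interact input activates that object on press and deactivates it on release, pausing target selection while held.
; Tick also calls health regeneration and drives a dynamic camera material from health; P deals test damage.
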(event EventBeginPlay
  ;[0 1 0.9246 0.172 11] On Begin Play
  ;;[0.1864 0.7469 1 1 8] Post Processing
  (CallFunction|SetMaterialtoPostProcess))

(event EventTick
  (params (DeltaSeconds :type Float%20%28single-precision%29))
  ;[1 1 1 1 11] Update
  (CallFunction|CheckInteractableObjects)
  (Class|HouseWarriorsCharacter|CanRegenerateHealth DeltaSeconds)
  (CallFunction|ControlUIHealth)
  (CallFunction|CheckGroundedStatus))

(event Collision|EventActorBeginOverlap
  (params (OtherActor :type Actor%20Object%20Reference))
  ;[1 0.8389 0] Object Collision Interation
  (bind _asinteractable_bp (Utilities|Casting|CastToInteractable_BP OtherActor))
  (CallFunction|CheckandAddObjects _asinteractable_bp))

(event Input|ActionEvents|InputActionInteract
  (params (Key :type Key%20Structure))
  (bind _currentinteractableobject (Variables|Default|GetCurrentInteractableObject))
  ;[0.7423 1 0.02228] Interact
  (:Pressed
    (Utilities|IsValid _currentinteractableobject
      (:Is%20Valid
        (Default|Activate _currentinteractableobject)
        (Variables|Default|SetactiveInteractableObject _currentinteractableobject))))
  (:Released
    (Utilities|IsValid (Variables|Default|GetactiveInteractableObject)
      (:Is%20Valid
        (Default|Deactivate (Variables|Default|GetactiveInteractableObject))
        (Variables|Default|SetactiveInteractableObject 0)))))

(event Input|KeyboardEvents|P
  (params (Key :type Key%20Structure))
  ;[1 0.01675 0 1 11] Current test for dealing damage
  (:Pressed
    (Class|HouseWarriorsCharacter|DealDamage 10)))

(fn ConstructionScript)

(fn ActivateInteractable
  (params (Actor :type Actor%20Object%20Reference))
  (bind _asbase_activator (Utilities|Casting|CastToBaseActivator Actor))
  (Default|Activate _asbase_activator))

(fn SetMaterialtoPostProcess
  (bind _returnvalue (Rendering|Material|CreateDynamicMaterialInstance (Variables|Default|GetScreenDamageMaterial) "None" :!class /Script/Engine.KismetMaterialLibrary))
  (bind _output_get (Variables|Default|SetDynamicScreenDamageMaterial _returnvalue))
  (Rendering|AddorUpdateBlendable (Variables|Default|GetFollowCamera) _output_get 1.0 :!class /Script/Engine.CameraComponent)
  (return))

(fn ControlUIHealth
  (Utilities|IsValid (Variables|Default|GetDynamicScreenDamageMaterial)
    (:Is%20Valid
      (bind _isactivated (Class|HouseWarriorsCharacter|UIHealth))
      (Rendering|Material|SetScalarParameterValue (Variables|Default|GetDynamicScreenDamageMaterial) "B_Density" _isactivated :!class /Script/Engine.MaterialInstanceDynamic)
      (Variables|/Script/Engine.CameraComponent|SetPostProcessBlendWeight (Variables|Default|GetFollowCamera) _isactivated)
      (return))))

(fn CheckInteractableObjects
  (bind _interactableobjects_arr (Variables|Default|GetInteractableObjects_arr))
  (bind _objecttoremove (Variables|Default|GetobjectToRemove))
  (if (not (Utilities|IsValid (Variables|Default|GetactiveInteractableObject)))
    (if (not (<= (Utilities|Array|Length (Variables|Default|GetInteractableObjects_arr)) 0))
      (Utilities|IsValid (Variables|Default|GetCurrentInteractableObject)
        (:Is%20Valid
          (Default|DeactivateGlow (Variables|Default|GetCurrentInteractableObject)))
        (:Is%20Not%20Valid
          _))
      (Variables|Default|SetCurrentInteractableObject 0)
      (for _array_element (Variables|Default|GetInteractableObjects_arr)
        (Utilities|IsValid _array_element
          (:Is%20Valid
            (if (and (< (Utilities|CalculateAngle _array_element) (Variables|Default|GetMinAngleToInteractable)) (<= (Transformation|GetDistanceTo _array_element self) (Variables|Default|GetMaxDistanceToInteract)))
              (Utilities|IsValid (Variables|Default|GetCurrentInteractableObject)
                (:Is%20Valid
                  (if (< (Utilities|CalculateAngle _array_element) (Utilities|CalculateAngle (Variables|Default|GetCurrentInteractableObject)))
                    (Variables|Default|SetCurrentInteractableObject _array_element :!label _label)))
                (:Is%20Not%20Valid
                  (goto _label)))))))
      (Utilities|IsValid _objecttoremove
        (:Is%20Valid
          (Default|DeactivateGlow _objecttoremove)
          (Utilities|Array|RemoveItem _interactableobjects_arr _objecttoremove))
        (:Is%20Not%20Valid
          _))
      (for _array_element_2 _interactableobjects_arr
        (if (== _array_element_2 (Variables|Default|GetCurrentInteractableObject))
          (Default|ActivateGlow _array_element_2)
          (else
            (Default|DeactivateGlow _array_element_2))))
      (return)
      (else
        _)))
  (return))

(fn CheckandAddObjects
  (params (Interactable :type Interactable%20BP%20Object%20Reference))
  (for _array_element (Variables|Default|GetInteractableObjects_arr)
    (if (== Interactable _array_element)
      (LocalVariables|SetbHasDuplicate true)))
  (if (LocalVariables|GetbHasDuplicate)
    (return)
    (else
      (Utilities|Array|Add (Variables|Default|GetInteractableObjects_arr) Interactable)
      (return))))

(fn CheckGroundedStatus
  (bind _cameraboom (Variables|Default|GetCameraBoom))
  (if (AI|Components|NavMovement|IsMovingonGround (Variables|Character|GetCharacterMovement))
    (Variables|/Script/Engine.SpringArmComponent|SetbEnableCameraLag _cameraboom true)
    (else
      (Variables|/Script/Engine.SpringArmComponent|SetbEnableCameraLag _cameraboom true)))
  (return))