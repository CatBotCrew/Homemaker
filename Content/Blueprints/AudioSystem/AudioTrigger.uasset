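; Trigger volume that plays two radio voice lines when the player character walks into its box.
; The overlap event plays the first cue on the referenced Radio, waits through a fixed delay, then plays the second.
; A Locked flag prevents later replays but is set only after the second cue starts, so re-entering during the delay can replay the first line.
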(event OnComponentBeginOverlap(Box)
  (params (OverlappedComponent :type Primitive%20Component%20Object%20Reference) (OtherActor :type Actor%20Object%20Reference) (OtherComp :type Primitive%20Component%20Object%20Reference) (OtherBodyIndex :type Integer) (bFromSweep :type Boolean) (SweepResult :type Hit%20Result%20Structure%20%28by%20ref%29))
  (if (== OtherActor (Game|GetPlayerCharacter 0))
    (if (not (Variables|Default|Getlocked))
      (Default|PlaySound (Variables|Default|Getradio) "/Game/Audio/Radio/VoiceLines/VoiceLine_1_Cue.VoiceLine_1_Cue")
      (Utilities|FlowControl|Delay 1e+01)
      (Default|PlaySound (Variables|Default|Getradio) "/Game/Audio/Radio/VoiceLines/VoiceLine_2_Cue.VoiceLine_2_Cue")
      (Variables|Default|Setlocked true))))

(fn ConstructionScript)