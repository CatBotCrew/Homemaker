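; Base Blueprint for openable doors that swing 90 degrees around a pivot when activated, optionally locked behind a key.
; On activation, KeyCheck looks for the required KeyID in the game instance's held keys, printing a temporary warning when it is missing.
; Activation sets a target rotation and an open or close flag, which Tick uses to interpolate the pivot via the SetDoor macro until nearly aligned, then flips IsOpen.
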(event EventOnActivation
  (bind _doorpivot (Variables|Default|GetDoorPivot))
  (bind _returnvalue (Math|Vector|GetForwardVector _doorpivot))
  (bind _returnvalue_2 (Math|Vector|GetUpVector _doorpivot))
  (bind _passed (CallFunction|KeyCheck))
  (if _passed
    (if (Variables|Default|GetisOpen)
      (if (not (Variables|Default|GetcloseDoor))
        (Variables|Default|SetcloseDoor true)
        (Variables|Default|SettargetRotation (Math|Conversions|RotationFromXVector (Math|Vector|RotateVectorAroundAxis _returnvalue 9e+01 _returnvalue_2))))
      (elif (not (Variables|Default|GetopenDoor))
        (Variables|Default|SetopenDoor true)
        (Variables|Default|SettargetRotation (Math|Conversions|RotationFromXVector (Math|Vector|RotateVectorAroundAxis _returnvalue -9e+01 _returnvalue_2)))))))

(event EventTick
  (params (DeltaSeconds :type Float%20%28single-precision%29))
  (if (Variables|Default|GetisOpen)
    (if (Variables|Default|GetcloseDoor)
      (Utilities|SetDoor
        (:Finished
          (Variables|Default|SetisOpen false)
          (Variables|Default|SetcloseDoor false))))
    (elif (Variables|Default|GetopenDoor)
      (Utilities|SetDoor
        (:Finished
          (Variables|Default|SetisOpen true)
          (Variables|Default|SetopenDoor false))))))

(fn ConstructionScript
  (|CallParentFunction))

(fn KeyCheck
  (if (Variables|Default|GetrequresKey)
    (bind _ashomemaker__gi (Utilities|Casting|CastToHomemaker-GI (Game|GetGameInstance))
      (:then
        (for _array_element (Variables|/Game/Blueprints/Homemaker-GI.Homemaker-GI_C|GetheldKeys _ashomemaker__gi)
          (if (Utilities|Enum|Equal(Enum) _array_element (Variables|Default|GetkeyID))
            (return true)))
        ;[1 1 1] Temporary Key Warning
        (Development|PrintString "This door is locked, and you don't have correct the key!" true true "(R=1.000000,G=0.000000,B=0.011301,A=1.000000)" 5.0)
        (return false))
      (:CastFailed
        (Development|PrintString "Game Instance Not Set!" true true "(R=1.000000,G=0.000000,B=0.011301,A=1.000000)" 5.0)))
    (else
      (return true))))