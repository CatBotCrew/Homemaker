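; BaseActivator is a base Blueprint for activators, with empty OnActivation and AfterActivation hooks.
; Activate calls OnActivation directly, or, when flagged as animated, sets the skeletal mesh's animation rate, plays the animation once and calls it after a delay.
; An animation already playing blocks reactivation, while a missing animation still waits out the delay.
; Deactivate simply calls AfterActivation.
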(event EventActivate
  (bind _returnvalue (Actor|GetComponentbyClass "/Script/Engine.SkeletalMeshComponent"))
  (if (Variables|Default|GetHasAnmimation)
    (Variables|/Script/Engine.SkeletalMeshComponent|SetGlobalAnimRateScale _returnvalue (Variables|Default|GetAnimationSpeed))
    (Utilities|IsValid (Variables|Default|GetAnimation)
      (:Is%20Valid
        (if (not (Audio|Components|Audio|IsPlaying _returnvalue))
          (Components|Animation|PlayAnimation _returnvalue (Variables|Default|GetAnimation) false)
          (Utilities|FlowControl|Delay (Variables|Default|GetAnimationDelay) :!label _label)
          (CallFunction|OnActivation)))
      (:Is%20Not%20Valid
        (goto _label)))
    (else
      (CallFunction|OnActivation))))

(event EventDeactivate
  (CallFunction|AfterActivation))

(fn ConstructionScript)

(fn OnActivation)

(fn AfterActivation)