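; Base bounce actor that launches the third-person character on overlap, acting as either a launch pad or a trampoline.
; A boolean selects the mode, and both override the character's horizontal and vertical velocity.
; Launch pad mode builds a fixed velocity from directional strength variables.
; Trampoline mode keeps the overlapping actor's horizontal velocity and inverts its vertical velocity, scaled by a bounce multiplier.
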(event EventBeginPlay)

(event Collision|EventActorBeginOverlap
  (params (OtherActor :type Actor%20Object%20Reference))
  (bind _asthird_person_character_bp (Utilities|Casting|CastToThirdPersonCharacter_BP OtherActor))
  (if (Variables|Default|GetIsLaunchPadNotTrampoline)
    (Character|LaunchCharacter _asthird_person_character_bp (Utilities|LaunchPadBounce) true true)
    (else
      (Character|LaunchCharacter _asthird_person_character_bp (Utilities|TrampolineBounce OtherActor) true true))))

(event EventTick
  (params (DeltaSeconds :type Float%20%28single-precision%29)))

(fn ConstructionScript)