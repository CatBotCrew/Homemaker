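; Portal actor that teleports overlapping actors to its linked ExitPortal and shows a live view through it.
; On BeginPlay, the exit's scene capture writes to a new render target that feeds this portal's dynamic material.
; Each tick, its own capture copies the player camera's rotation and its position relative to the exit portal.
; Teleporting disables the exit portal, and a delayed end-overlap re-enables it to prevent bouncing back.
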(event EventBeginPlay
  (bind _returnvalue (Rendering|CreateRenderTarget2D 1920 1080 "RTF_RGBA16f"))
  (bind _output_get (Variables|/Script/Engine.SceneCaptureComponent2D|SetTextureTarget (Actor|GetComponentbyClass (Variables|Default|GetExitPortal) "/Script/Engine.SceneCaptureComponent2D") _returnvalue))
  (bind _returnvalue_2 (Rendering|Material|CreateDynamicMaterialInstance (Variables|Default|GetPortal) 0 "/Game/Blueprints/Portals/PortalMaterial.PortalMaterial" "DynamicPortalMaterial" :!class /Script/Engine.PrimitiveComponent))
  (Rendering|Material|SetTextureParameterValue _returnvalue_2 "PortalTexture" _output_get))

(event EventTick
  (params (DeltaSeconds :type Float%20%28single-precision%29))
  (bind _returnvalue (Game|GetPlayerCameraManager 0))
  (bind _transformcomponent (Variables|/Script/Engine.PlayerCameraManager|GetTransformComponent _returnvalue))
  ;[1 1 1] View Updating
  (Transformation|SetWorldLocationAndRotation (Variables|Default|GetPortalCapture) (+ (- (Transformation|GetWorldLocation (Variables|Default|GetDefaultSceneRoot)) (Transformation|GetWorldLocation (Variables|Portal_C|GetDefaultSceneRoot (Variables|Default|GetExitPortal)))) (Transformation|GetWorldLocation _transformcomponent)) (Transformation|GetWorldRotation _transformcomponent) false false))

(event Collision|EventActorBeginOverlap
  (params (OtherActor :type Actor%20Object%20Reference))
  (bind _exitportal (Variables|Default|GetExitPortal))
  ;[1 1 1] Teleportation
  (if (Variables|Default|GetCanTeleport)
    (Variables|Portal_C|SetCanTeleport _exitportal false)
    (Transformation|SetWorldLocation (Variables|/Script/Engine.Actor|GetRootComponent OtherActor) (Transformation|GetWorldLocation (Variables|Portal_C|GetDefaultSceneRoot _exitportal)) false false)))

(event Collision|EventActorEndOverlap
  (params (OtherActor :type Actor%20Object%20Reference))
  ;[1 1 1] Teleportation
  (Utilities|FlowControl|Delay 0.4)
  (Variables|Default|SetCanTeleport true))

(fn ConstructionScript)