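; Test trigger actor that plays a radio voice line, identified by VoiceID, when the player character overlaps it.
; It asks RadioLineTrigger to play immediately, or after a Tick-driven TimerSec countdown when IsTimedTrigger is set.
; If the request fails, it copies the active voice line's TimerSec and retries when that countdown expires.
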(event EventBeginPlay)

(event Collision|EventActorBeginOverlap
  (params (OtherActor :type Actor%20Object%20Reference))
  (Utilities|Casting|CastToBP_PlayerCharacter OtherActor)
  (if (Variables|Default|GetIsTimedTrigger)
    (Variables|Default|SetIsTimerReady true)
    (else
      (bind _iscomplete (Default|TriggerVoiceLine (Variables|Default|GetRadioLineTrigger) (Variables|Default|GetVoiceID)))
      (if (not _iscomplete)
        (Variables|Default|SetTimer%20%28Sec%29 (.timersec (Variables|/Game/Blueprints/RadioVoiceLines/BP_RadioLineTrigger.BP_RadioLineTrigger_C|GetcurrentActiveVoiceLine (Variables|Default|GetRadioLineTrigger))))
        (Variables|Default|SetIsTimerReady true)))))

(event EventTick
  (params (DeltaSeconds :type Float%20%28single-precision%29))
  (if (Variables|Default|GetIsTimerReady)
    (bind _output_get (Variables|Default|SetTimer%20%28Sec%29 (- (Variables|Default|GetTimer%20%28Sec%29) DeltaSeconds)))
    (if (<= _output_get 0.0)
      (Variables|Default|SetIsTimerReady false)
      (bind _iscomplete (Default|TriggerVoiceLine (Variables|Default|GetRadioLineTrigger) (Variables|Default|GetVoiceID)))
      (if (not _iscomplete)
        (Variables|Default|SetTimer%20%28Sec%29 (.timersec (Variables|/Game/Blueprints/RadioVoiceLines/BP_RadioLineTrigger.BP_RadioLineTrigger_C|GetcurrentActiveVoiceLine (Variables|Default|GetRadioLineTrigger))))
        (Variables|Default|SetIsTimerReady true)))))

(fn ConstructionScript)