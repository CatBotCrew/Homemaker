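; Voice line trigger actor that plays indexed radio lines from its VoiceLines array through the level's Radio actors.
; TriggerVoiceLine looks up a line by ID, skips completed ones and marks non-repeatable lines complete; the repeat timer is still a TODO.
; PlayLine refreshes the radio list via CheckRadios, then plays the sound at every radio's location, falling back to 2D audio when none exist.
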(event EventBeginPlay
  (CallFunction|CheckRadios))

(event Collision|EventActorBeginOverlap
  (params (OtherActor :type Actor%20Object%20Reference)))

(event EventTick
  (params (DeltaSeconds :type Float%20%28single-precision%29)))

(fn ConstructionScript)

(fn CheckRadios
  (bind _outactors (Actor|GetAllActorsOfClass "/Game/Blueprints/Objects/Radio.Radio_C"))
  (Utilities|IsValid (Utilities|Array|Get(acopy) _outactors)
    (:Is%20Valid
      (Variables|Default|SetRadios_arr _outactors)
      (return true))
    (:Is%20Not%20Valid
      (return false) ; No Radios are available in this chapter/room
    )))

(fn TriggerVoiceLine
  (params (Line%20ID :type Integer))
  (bind _output_get (LocalVariables|SetLineID Line%20ID))
  (if (Utilities|Array|IsValidIndex (Variables|Default|GetVoiceLines) Line%20ID)
    (bind _output_get_2 (Variables|Default|SetcurrentActiveVoiceLine (Utilities|Array|Get(acopy) (Variables|Default|GetVoiceLines) _output_get)))
    (if (.bislinecomplete _output_get_2)
      (return false) ; Voice line already completed
      (elif (.bisrepeatable _output_get_2)
        ;[0.162 1 0.2301 1 12] Play and Restart Timer
        (CallFunction|PlayLine (Variables|Default|GetcurrentActiveVoiceLine))
        (return false) ; TODO: Timer
        (else
          ;[1 0.1135 0.003805 1 12] Play and Set Voice Line Complete
          (CallFunction|PlayLine (Variables|Default|GetcurrentActiveVoiceLine))
          (bind _output_get_3 (Variables|Default|SetcurrentActiveVoiceLine (Utilities|Struct|MakeVoiceLine (.voiceline (Variables|Default|GetcurrentActiveVoiceLine)) (.triggerid (Variables|Default|GetcurrentActiveVoiceLine)) (.timersec (Variables|Default|GetcurrentActiveVoiceLine)) (.bisrepeatable (Variables|Default|GetcurrentActiveVoiceLine)) true)))
          (Utilities|Array|SetArrayElem (Variables|Default|GetVoiceLines) (LocalVariables|GetLineID) _output_get_3)
          (return true))))
    (else
      (Development|PrintString "Voice line not available" true true "(R=1.000000,G=0.000000,B=0.018187,A=1.000000)"))))

(fn PlayLine
  (params (VoiceLine :type Voice%20Line%20Structure))
  (bind _isavailable (CallFunction|CheckRadios))
  (if _isavailable
    ;[1 0.3615 0.4213 1 12] Might want to have a play function in radio bp and call here.
    (for _array_element (Variables|Default|GetRadios_arr)
      (Audio|PlaySoundatLocation (.voiceline VoiceLine) (Transformation|GetActorLocation _array_element) "0, 0, 0" 1.0 1.0 0.0 0 0 0))
    (else
      (Audio|PlaySound2D (.voiceline VoiceLine) 1.0 1.0 0.0 0 0) ; Play's Sound at UI if there is no Radios to play at.
    ))
  (return))